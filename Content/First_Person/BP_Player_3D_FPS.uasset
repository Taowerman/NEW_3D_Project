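; First-person shooter player Blueprint handling movement, look, jump and shooting through Enhanced Input actions.
; Movement follows the control rotation's yaw, look input turns the controller at a set rotation speed, and jumping plays a sound.
; Shooting is hitscan: a camera-forward Visibility trace with persistent debug drawing feeds point damage to the hit actor.
; Each shot plays two sounds and pulses force feedback, regardless of whether it hits.
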(event Input|EnhancedActionEvents|EnhancedInputActionIA_Move
  (params (ActionValue :type Vector%202D%20Structure) (ElapsedSeconds :type Float%20%28double-precision%29) (TriggeredSeconds :type Float%20%28double-precision%29) (InputAction :type Input%20Action%20Object%20Reference :default "/Game/Input/Actions/IA_Move.IA_Move"))
  (bind (_x _y) (Math|Vector2D|BreakVector2D ActionValue))
  (bind _returnvalue (Pawn|GetControlRotation :!class /Script/Engine.Pawn))
  (bind _yaw (Math|Rotator|BreakRotator _returnvalue))
  (bind _returnvalue_2 (Math|Rotator|MakeRotator 0.0 0.0 _yaw))
  (Pawn|Input|AddMovementInput (Math|Vector|GetRightVector _returnvalue_2) (* _x (Variables|Default|GetMovementSpeed)) false) ; left/right
  (Pawn|Input|AddMovementInput (Math|Vector|GetForwardVector _returnvalue_2) (* _y (Variables|Default|GetMovementSpeed)) false) ; forward/backward
)

(event Input|EnhancedActionEvents|EnhancedInputActionIA_Jump
  (params (ActionValue :type Boolean) (ElapsedSeconds :type Float%20%28double-precision%29) (TriggeredSeconds :type Float%20%28double-precision%29) (InputAction :type Input%20Action%20Object%20Reference :default "/Game/Input/Actions/IA_Jump.IA_Jump"))
  (:Started
    (Character|Jump)
    (Audio|PlaySoundatLocation "/Game/Audio/SoundEffects/jump_sound.jump_sound" "0, 0, 0" "0, 0, 0" 3.0 1.0 0.0 0 0 0 0)))

(event Input|EnhancedActionEvents|EnhancedInputActionIA_Look
  (params (ActionValue :type Vector%202D%20Structure) (ElapsedSeconds :type Float%20%28double-precision%29) (TriggeredSeconds :type Float%20%28double-precision%29) (InputAction :type Input%20Action%20Object%20Reference :default "/Game/Input/Actions/IA_Look.IA_Look"))
  (bind (_x _y) (Math|Vector2D|BreakVector2D ActionValue))
  (Pawn|Input|AddControllerYawInput (* _x (Variables|Default|GetRotationSpeed)))
  (Pawn|Input|AddControllerPitchInput (* _y (Variables|Default|GetRotationSpeed))))

(event Input|EnhancedActionEvents|EnhancedInputActionIA_Shoot
  (params (ActionValue :type Float%20%28double-precision%29) (ElapsedSeconds :type Float%20%28double-precision%29) (TriggeredSeconds :type Float%20%28double-precision%29) (InputAction :type Input%20Action%20Object%20Reference :default "/Game/Input/Actions/IA_Shoot.IA_Shoot"))
  (bind _camera (Variables|Default|GetCamera))
  (bind _returnvalue (Transformation|GetWorldLocation _camera))
  (bind _returnvalue_2 (Math|Vector|GetForwardVector _camera))
  (:Started
    (bind _outhit (Collision|LineTraceByChannel _returnvalue (+ _returnvalue (* _returnvalue_2 (Variables|Default|GetShootRange))) "TraceTypeQuery1" false 0 "Persistent")) ; Line for bullet detection
    (Audio|PlaySoundatLocation "/Game/Audio/SoundEffects/damage_enemy.damage_enemy" "0, 0, 0" "0, 0, 0" 3.0 1.0 0.0 0 0 0 0)
    (Game|Damage|ApplyPointDamage (.HitActor (Collision|BreakHitResult _outhit)) (Variables|Default|GetDamageAmount) _returnvalue_2 _outhit 0 self)
    (Audio|PlaySoundatLocation "/Game/Audio/SoundEffects/Boom5.Boom5" (Transformation|GetActorLocation) "0, 0, 0" 1.0 1.0 0.0 0 0 0 0)
    (Game|Feedback|PlayDynamicForceFeedback (Game|GetPlayerController 0) 1.0 0.1 true true true true)))

(event EventBeginPlay)

(event Collision|EventActorBeginOverlap
  (params (OtherActor :type Actor%20Object%20Reference)))

(event EventTick
  (params (DeltaSeconds :type Float%20%28single-precision%29)))

(fn ConstructionScript)